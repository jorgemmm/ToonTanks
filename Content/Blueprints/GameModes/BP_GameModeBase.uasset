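; Base game mode Blueprint that manages the on-screen UI at the start and end of a match.
; GameStart shows a start widget fed with StartDelay, then adds and stores the HUD beneath it after a separate hardcoded delay.
; GameOver removes that HUD and shows an end screen that receives whether the player won.
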(event `self.GameStart`
  (`|ExecutionSequence`
    (:`then_0`
      (bind _returnvalue (`|CreateWidget` "/Game/Blueprints/Widgets/WBP_GameStart.WBP_GameStart_C" (cast `/Game/Blueprints/PlayerControllers/BP_PlayerController` (`GameplayStatics.GetPlayerController` 0) :!pure true)))
      (`/Game/Blueprints/Widgets/WBP_GameStart.SetStartDelay` _returnvalue (`self.StartDelay`))
      (`UserWidget.AddToViewport` _returnvalue 1))
    (:`then_1`
      (`KismetSystemLibrary.Delay` 5.0)
      (bind _returnvalue_2 (`|CreateWidget` "/Game/Blueprints/Widgets/WBP_HUD.WBP_HUD_C"))
      (bind _output_get (set `self.WB_HUDRef` _returnvalue_2))
      (`UserWidget.AddToViewport` _returnvalue_2 0)
      (`UserWidget.AddToViewport` _output_get 0))))

(event `self.GameOver`
  (params (PlayerWon :type Boolean))
  (`|ExecutionSequence`
    (:`then_0`
      (`Widget.RemoveFromParent` (`self.WB_HUDRef`)))
    (:`then_1`
      (bind _returnvalue (`|CreateWidget` "/Game/Blueprints/Widgets/WBP_GameEnd.WBP_GameEnd_C" (cast `/Game/Blueprints/PlayerControllers/BP_PlayerController` (`GameplayStatics.GetPlayerController` 0) :!pure true)))
      (`/Game/Blueprints/Widgets/WBP_GameEnd.SetPlayerWin` _returnvalue PlayerWon)
      (`UserWidget.AddToViewport` _returnvalue 0))))

(fn `UserConstructionScript`)